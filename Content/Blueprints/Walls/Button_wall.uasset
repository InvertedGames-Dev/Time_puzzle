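; Button-driven wall Blueprint that slides its Wall component vertically when triggered and returns it when the trigger is released.
; The OldWall flag picks the direction: up toward 300, or otherwise down toward -600, returning toward zero on release.
; Tick feeds paired Gate nodes that the trigger events open and close, moving the wall in fixed, clamped per-frame steps independent of delta time.
; The construction script sizes the wall from width and height variables.
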(event `/Game/Blueprints/Triggers/BPI_Trigger.Trigger On`
  (bind _returnvalue (- (`self.Current Z`) 5.0))
  (bind _returnvalue_2 (- (`self.Current Z`) 5.0))
  (bind _returnvalue_3 (+ (`self.Current Z`) 5.0))
  (bind _returnvalue_4 (+ (`self.Current Z`) 5.0))
  (if (`self.Old Wall?`)
    (`|ExecutionSequence`
      (:`then_0`
        (goto _label_2 :!via `Close`))
      (:`then_1`
        (goto _label :!via `Open`)))
    (else
      (`|ExecutionSequence`
        (:`then_0`
          (goto _label_4 :!via `Close`))
        (:`then_1`
          (goto _label_3 :!via `Open`))))))

(event `self.ReceiveTick`
  (params (DeltaSeconds :type "Float (single-precision)"))
  (bind _returnvalue (- (`self.Current Z`) 5.0))
  (bind _returnvalue_2 (- (`self.Current Z`) 5.0))
  (bind _returnvalue_3 (+ (`self.Current Z`) 5.0))
  (bind _returnvalue_4 (+ (`self.Current Z`) 5.0))
  (if (`self.Old Wall?`)
    (`|ExecutionSequence`
      (:`then_0`
        (`/Engine/EditorBlueprintResources/StandardMacros.Gate` true :!label _label
          (:`Exit`
            (if (<= _returnvalue_4 300.0)
              (set `self.Current Z` _returnvalue_4)
              (`SceneComponent.K2_SetRelativeLocation` (`self.Wall`) (`KismetMathLibrary.MakeVector` 0.0 0.0 (`self.Current Z`)) false false)))))
      (:`then_1`
        (`/Engine/EditorBlueprintResources/StandardMacros.Gate` true :!label _label_2
          (:`Exit`
            (if (>= _returnvalue_2 0.0)
              (set `self.Current Z` _returnvalue_2)
              (`SceneComponent.K2_SetRelativeLocation` (`self.Wall`) (`KismetMathLibrary.MakeVector` 0.0 0.0 (`self.Current Z`)) false false))))))
    (else
      (`|ExecutionSequence`
        (:`then_0`
          (`/Engine/EditorBlueprintResources/StandardMacros.Gate` true :!label _label_3
            (:`Exit`
              (if (>= _returnvalue -600.0)
                (set `self.Current Z` _returnvalue)
                (`SceneComponent.K2_SetRelativeLocation` (`self.Wall`) (`KismetMathLibrary.MakeVector` 0.0 0.0 (`self.Current Z`)) false false)))))
        (:`then_1`
          (`/Engine/EditorBlueprintResources/StandardMacros.Gate` true :!label _label_4
            (:`Exit`
              (if (<= _returnvalue_3 0.0)
                (set `self.Current Z` _returnvalue_3)
                (`SceneComponent.K2_SetRelativeLocation` (`self.Wall`) (`KismetMathLibrary.MakeVector` 0.0 0.0 (`self.Current Z`)) false false)))))))))

(event `/Game/Blueprints/Triggers/BPI_Trigger.Trigger Off`
  (if (`self.Old Wall?`)
    (`|ExecutionSequence`
      (:`then_0`
        (goto _label :!via `Close`))
      (:`then_1`
        (goto _label_2 :!via `Open`)))
    (else
      (`|ExecutionSequence`
        (:`then_0`
          (goto _label_3 :!via `Close`))
        (:`then_1`
          (goto _label_4 :!via `Open`))))))

(fn `UserConstructionScript`
  (`SceneComponent.SetRelativeScale3D` (`self.Wall`) (`KismetMathLibrary.MakeVector` (`self.Wall Scale X`) 0.2 (`self.Wall scale Z`))))