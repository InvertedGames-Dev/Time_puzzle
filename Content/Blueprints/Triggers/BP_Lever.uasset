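; BP_Lever is an interactable two-state lever that switches a linked TriggeredItem on or off.
; Sphere overlap shows or hides the FirstPersonCharacter's HUD use prompt and sets or clears that character's LeverReference to this lever.
; Interact toggles between LeverUp and LeverDown, which rotate the lever and recolor its point light red or green, then sends TriggeredItem the matching off or on message.
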(event `self.Sphere.OnComponentBeginOverlap`
  (params (OverlappedComponent :type "PrimitiveComponent Object Reference") (OtherActor :type "Actor Object Reference") (OtherComp :type "PrimitiveComponent Object Reference") (OtherBodyIndex :type Integer) (bFromSweep :type Boolean) (SweepResult :type "HitResult Structure (by ref)"))
  (bind _asfirst_person_character (cast `/Game/FirstPersonBP/Blueprints/FirstPersonCharacter` OtherActor))
  (`/Game/UI/HUD.Event Show Use Text` (`/Game/FirstPersonBP/Blueprints/FirstPersonCharacter.Hud Reference` _asfirst_person_character))
  (set `/Game/FirstPersonBP/Blueprints/FirstPersonCharacter.Lever Reference` self _asfirst_person_character))

(event `self.Sphere.OnComponentEndOverlap`
  (params (OverlappedComponent :type "PrimitiveComponent Object Reference") (OtherActor :type "Actor Object Reference") (OtherComp :type "PrimitiveComponent Object Reference") (OtherBodyIndex :type Integer))
  (bind _asfirst_person_character (cast `/Game/FirstPersonBP/Blueprints/FirstPersonCharacter` OtherActor))
  (`/Game/UI/HUD.Event Hide Use Text` (`/Game/FirstPersonBP/Blueprints/FirstPersonCharacter.Hud Reference` _asfirst_person_character))
  (set `/Game/FirstPersonBP/Blueprints/FirstPersonCharacter.Lever Reference` null _asfirst_person_character))

(event `Lever Up`
  (`SceneComponent.K2_SetRelativeTransform` (`self.Lever`) (`KismetMathLibrary.MakeTransform` (0.0 0.0 0.0)) true false)
  (set `self.Lever Up?` true)
  (`LightComponent.SetLightColor` (`self.PointLight`) (struct :`R` 1.0 :`A` 1.0) true))

(event `Interact`
  (bind _triggered_item (`self.Triggered Item`))
  (if (`self.Lever Up?`)
    (`self.Lever Down`)
    (message `/Game/Blueprints/Triggers/BPI_Trigger.Trigger On` _triggered_item)
    (else
      (`self.Lever Up`)
      (message `/Game/Blueprints/Triggers/BPI_Trigger.Trigger Off` _triggered_item))))

(event `Lever Down`
  (`SceneComponent.K2_SetRelativeTransform` (`self.Lever`) (`KismetMathLibrary.MakeTransform` (0.0 0.0 0.0) (struct :`Yaw` -180.0)) true false)
  (set `self.Lever Up?` false)
  (`LightComponent.SetLightColor` (`self.PointLight`) (struct :`G` 1.0 :`B` 0.009126 :`A` 1.0) true))

(fn `UserConstructionScript`)