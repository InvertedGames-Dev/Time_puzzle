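; BP_Big_Button is a floor-style trigger button that activates its TriggeredObjects when FirstPersonCharacter or a Time_Object overlaps its box.
; Pressing lowers the button, turns its light and base glow orange, sends TriggerOnMessage to each object and opens a gate.
; End overlap passes through that gate to restore the raised blue state, send TriggerOffMessage and set Reset on any Catapult.
; Other overlapping actors close the gate.
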(event `self.Box.OnComponentBeginOverlap`
  (params (OverlappedComponent :type "PrimitiveComponent Object Reference") (OtherActor :type "Actor Object Reference") (OtherComp :type "PrimitiveComponent Object Reference") (OtherBodyIndex :type Integer) (bFromSweep :type Boolean) (SweepResult :type "HitResult Structure (by ref)"))
  (cast `/Game/FirstPersonBP/Blueprints/FirstPersonCharacter` OtherActor
    (:`then`
      (`self.Button Down`))
    (:`CastFailed`
      (cast `/Game/Blueprints/Time_Objects/Time_Object` OtherActor
        (:`then`
          (`self.Button Down`))
        (:`CastFailed`
          (goto _label :!via `Close`)))))
  (`|ExecutionSequence`
    (:`then_0`
      (goto _label :!via `Open`))
    (:`then_1`
      (for _array_element (`self.Triggered Objects`)
        (message `/Game/Blueprints/Triggers/BPI_Trigger.Trigger On` _array_element)))))

(event `self.Box.OnComponentEndOverlap`
  (params (OverlappedComponent :type "PrimitiveComponent Object Reference") (OtherActor :type "Actor Object Reference") (OtherComp :type "PrimitiveComponent Object Reference") (OtherBodyIndex :type Integer))
  (`/Engine/EditorBlueprintResources/StandardMacros.Gate` true :!label _label
    (:`Exit`
      (`self.Button Up`)
      (for _array_element (`self.Triggered Objects`)
        (message `/Game/Blueprints/Triggers/BPI_Trigger.Trigger Off` _array_element)
        (bind _ascatapult (cast `/Game/Blueprints/Catapult` _array_element))
        (set `/Game/Blueprints/Catapult.Reset?` true _ascatapult)))))

(fn `Button Down`
  (`SceneComponent.K2_SetRelativeLocation` (`self.Button`) (0.0 0.0 -15.0) false false)
  (set `self.Button Activated` true)
  (`LightComponent.SetLightColor` (`self.PointLight`) (struct :`R` 1.0 :`G` 0.301961 :`A` 1.0) true)
  (`PrimitiveComponent.SetMaterial` (`self.Button Base`) 2 "/Game/Props/Big_button/Button_Glow_Orange.Button_Glow_Orange"))

(fn `Button Up`
  (`SceneComponent.K2_SetRelativeLocation` (`self.Button`) (0.0 0.0 -5.0) false false)
  (set `self.Button Activated` false)
  (`LightComponent.SetLightColor` (`self.PointLight`) (struct :`R` 0.113725 :`G` 0.690196 :`B` 0.87451 :`A` 1.0) true)
  (`PrimitiveComponent.SetMaterial` (`self.Button Base`) 2 "/Game/Props/Big_button/Button_Glow_Blue.Button_Glow_Blue"))

(fn `UserConstructionScript`)