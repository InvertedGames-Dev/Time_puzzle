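; Physics object that responds to the player's time rewind and stop powers according to its type: Rewindable, Stoppable or Universal.
; While simulation is enabled, Tick records transforms and velocities (packed into transforms), skipping roughly unchanged samples, then pops them to rewind.
; Time stop disables physics on Stoppable and Universal objects, and materials reflect type and activity.
; Reset events or falling below a height threshold restore the original transform and clear history.
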(event `self.ReceiveBeginPlay`
  (bind _asfirst_person_character (cast `/Game/FirstPersonBP/Blueprints/FirstPersonCharacter` (`GameplayStatics.GetPlayerCharacter` 0)))
  (set `self.Character Reference` _asfirst_person_character)
  (`PrimitiveComponent.SetSimulatePhysics` (`self.StaticMesh`) false))

(event `self.ReceiveTick`
  (params (DeltaSeconds :type "Float (single-precision)"))
  (bind _character_reference (`self.Character Reference`))
  (bind _velocity_array (`self.Velocity Array`))
  (bind _staticmesh (`self.StaticMesh`))
  (bind _transform_array (`self.Transform Array`))
  (bind _staticmesh_2 (`self.StaticMesh`))
  (bind _object_type (`self.Object type`))
  (bind _object_type_2 (`self.Object type`))
  (bind _character_reference_2 (`self.Character Reference`))
  (bind _object_type_3 (`self.Object type`))
  (bind _object_type_4 (`self.Object type`))
  (bind _returnvalue (`KismetArrayLibrary.Array_LastIndex` _transform_array))
  (bind _returnvalue_2 (`KismetArrayLibrary.Array_LastIndex` _velocity_array))
  (bind _returnvalue_3 (`SceneComponent.K2_GetComponentToWorld` _staticmesh_2))
  (bind _stop_time (`/Game/FirstPersonBP/Blueprints/FirstPersonCharacter.Stop Time` _character_reference))
  (bind _reverse_time (`/Game/FirstPersonBP/Blueprints/FirstPersonCharacter.Reverse Time` _character_reference))
  (bind _output (`|GetArrayItem` _transform_array _returnvalue))
  (bind _returnvalue_4 (and _reverse_time (not _stop_time)))
  (`/Engine/EditorBlueprintResources/StandardMacros.Gate` true :!label _label
    (:`Exit`
      (set `self.Not moving` (and (`self.V not moving`) (`self.L not moving`)))
      (`|ExecutionSequence`
        (:`then_0`
          (if (or (`|EnumEquality` _object_type "NewEnumerator2") (`|EnumEquality` _object_type "NewEnumerator0"))
            (`|ExecutionSequence`
              (:`then_0`
                (if _returnvalue_4
                  (`SceneComponent.K2_SetWorldTransform` _staticmesh_2 _output false false)
                  (if (> _returnvalue 0)
                    (`KismetArrayLibrary.Array_Remove` _transform_array _returnvalue))
                  (elif (and _stop_time (or (`|EnumEquality` _object_type_3 "NewEnumerator1") (`|EnumEquality` _object_type_3 "NewEnumerator0")))
                    _
                    (elif (`self.Compare rough transforms` _output _returnvalue_3)
                      (set `self.L not moving` true)
                      (else
                        (`KismetArrayLibrary.Array_Add` _transform_array _returnvalue_3)
                        (set `self.L not moving` false))))))
              (:`then_1`
                (if _returnvalue_4
                  (`PrimitiveComponent.SetPhysicsLinearVelocity` _staticmesh_2 (.location (`|GetArrayItem` _velocity_array _returnvalue_2)) false "None")
                  (`PrimitiveComponent.SetPhysicsAngularVelocity` _staticmesh_2 (.scale (`|GetArrayItem` _velocity_array _returnvalue_2)) false "None")
                  (if (> _returnvalue_2 0)
                    (`KismetArrayLibrary.Array_Remove` _velocity_array _returnvalue_2))
                  (elif (not _stop_time)
                    (bind _returnvalue_5 (`PrimitiveComponent.GetPhysicsLinearVelocity` _staticmesh_2 "None"))
                    (bind _returnvalue_6 (`PrimitiveComponent.GetPhysicsAngularVelocity` _staticmesh_2 "None"))
                    (bind _returnvalue_7 (`KismetMathLibrary.MakeTransform` _returnvalue_5 (struct) _returnvalue_6))
                    (if (`self.Compare rough transforms` (`|GetArrayItem` _velocity_array _returnvalue_2) _returnvalue_7)
                      (set `self.V not moving` true)
                      (else
                        (`KismetArrayLibrary.Array_Add` _velocity_array _returnvalue_7)
                        (set `self.V not moving` false)))))))))
        (:`then_1`
          (`PrimitiveComponent.SetMaterial` (`self.StaticMesh`) 0 (select `bool` (or (`self.Not moving`) _reverse_time) :`false` (select `/Game/Blueprints/Time_Objects/Object_Type` _object_type_2 :`NewEnumerator0` "/Game/Blueprints/Time_Objects/Fragment_Active.Fragment_Active" :`NewEnumerator1` "/Game/Blueprints/Time_Objects/Freeze_Fragment_Dormant1.Freeze_Fragment_Dormant1" :`NewEnumerator2` "/Game/Blueprints/Time_Objects/Fragment_Active.Fragment_Active" :!type "Material Object Reference") :`true` (select `/Game/Blueprints/Time_Objects/Object_Type` _object_type_2 :`NewEnumerator0` "/Game/Blueprints/Time_Objects/U_Fragment_Dormant.U_Fragment_Dormant" :`NewEnumerator1` "/Game/Blueprints/Time_Objects/Freeze_Fragment_Dormant1.Freeze_Fragment_Dormant1" :`NewEnumerator2` "/Game/Blueprints/Time_Objects/Rewind_Fragment_Dormant.Rewind_Fragment_Dormant" :!type "Material Object Reference"))))
        (:`then_2`
          (bind _returnvalue_8 (`PrimitiveComponent.GetPhysicsLinearVelocity` (`self.StaticMesh`) "None"))
          (set `self.Velocity` _returnvalue_8)
          (if (or (`|EnumEquality` _object_type_4 "NewEnumerator1") (`|EnumEquality` _object_type_4 "NewEnumerator0"))
            (if (and (not (`/Game/FirstPersonBP/Blueprints/FirstPersonCharacter.Reverse Time` _character_reference_2)) (`/Game/FirstPersonBP/Blueprints/FirstPersonCharacter.Stop Time` _character_reference_2))
              (`PrimitiveComponent.SetSimulatePhysics` _staticmesh false)
              (else
                (`PrimitiveComponent.SetSimulatePhysics` _staticmesh true)))))
        (:`then_3`
          (`self.Reset if fallen off world`))))))

(event `Begin simulation`
  (goto _label :!via `Open`))

(event `End Simulation`
  (goto _label :!via `Close`))

(event `Reset objects`
  (bind _staticmesh (`self.StaticMesh`))
  (`PrimitiveComponent.SetSimulatePhysics` _staticmesh false)
  (`SceneComponent.K2_SetWorldTransform` (`self.StaticMesh`) (`self.Origin Transform`) false true)
  (`PrimitiveComponent.SetSimulatePhysics` _staticmesh true)
  (`KismetArrayLibrary.Array_Clear` (`self.Velocity Array`))
  (`KismetArrayLibrary.Array_Clear` (`self.Transform Array`)))

(fn `Compare rough transforms`
  (params (T1 :type "Transform Structure") (T2 :type "Transform Structure"))
  (returns (Equal :type Boolean))
  (return (and (and (== (`KismetMathLibrary.Round` (.x (.location T1))) (`KismetMathLibrary.Round` (.x (.location T2)))) (== (`KismetMathLibrary.Round` (.y (.location T1))) (`KismetMathLibrary.Round` (.y (.location T2)))) (== (`KismetMathLibrary.Round` (.z (.location T1))) (`KismetMathLibrary.Round` (.z (.location T2))))) (and (== (`KismetMathLibrary.Round` (.x (.scale T1))) (`KismetMathLibrary.Round` (.x (.scale T2)))) (== (`KismetMathLibrary.Round` (.y (.scale T1))) (`KismetMathLibrary.Round` (.y (.scale T2)))) (== (`KismetMathLibrary.Round` (.z (.scale T1))) (`KismetMathLibrary.Round` (.z (.scale T2))))))))

(fn `Draw Arrow to cube`
  (params (Cube :type "Actor Object Reference") (Arrow :type "ArrowComponent Object Reference"))
  (bind _returnvalue (- (`self.K2_GetActorLocation` Cube) (`self.K2_GetActorLocation`)))
  (`/Engine/EditorBlueprintResources/StandardMacros.IsValid` Cube
    (:`Is Valid`
      (`SceneComponent.K2_SetRelativeTransform` Arrow (`KismetMathLibrary.MakeTransform` (0.0 0.0 0.0) (`KismetMathLibrary.Conv_VectorToRotator` (`KismetMathLibrary.InverseTransformDirection` (`self.GetTransform`) _returnvalue)) (`KismetMathLibrary.MakeVector` (/ (`KismetMathLibrary.VSize` _returnvalue) 80.0) 1.0 1.0)) false false))))

(fn `Reset if fallen off world`
  (bind _staticmesh (`self.StaticMesh`))
  (bind (_returnvalue_x _returnvalue_y _returnvalue_z) (`KismetMathLibrary.BreakVector` (`SceneComponent.K2_GetComponentLocation` (`self.StaticMesh`))))
  (if (<= _returnvalue_z 10.0)
    (`PrimitiveComponent.SetSimulatePhysics` _staticmesh false)
    (`SceneComponent.K2_SetWorldTransform` (`self.StaticMesh`) (`self.Origin Transform`) false true)
    (`PrimitiveComponent.SetSimulatePhysics` _staticmesh true)
    (`KismetArrayLibrary.Array_Clear` (`self.Velocity Array`))
    (`KismetArrayLibrary.Array_Clear` (`self.Transform Array`))))

(fn `UserConstructionScript`
  (set `self.Origin Transform` (`SceneComponent.K2_GetComponentToWorld` (`self.StaticMesh`)))
  (`PrimitiveComponent.SetMaterial` (`self.StaticMesh`) 0 (select `/Game/Blueprints/Time_Objects/Object_Type` (`self.Object type`) :`NewEnumerator0` "/Game/Blueprints/Time_Objects/U_Fragment_Dormant.U_Fragment_Dormant" :`NewEnumerator1` "/Game/Blueprints/Time_Objects/Freeze_Fragment_Dormant1.Freeze_Fragment_Dormant1" :`NewEnumerator2` "/Game/Blueprints/Time_Objects/Rewind_Fragment_Dormant.Rewind_Fragment_Dormant" :!type "Material Object Reference")))