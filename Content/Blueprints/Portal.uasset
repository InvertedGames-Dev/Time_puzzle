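; Portal actor that acts as either an entrance or an exit, with particle template and light color set by IsExitPortal at construction.
; Player overlap with an exit starts physics and simulation on its Time_Object and HamsterBall arrays.
; An entrance with a valid TargetPortal teleports the player there, records it as SpawnPortal and stops those objects' simulation.
; Settosimulate runs the same branching logic, while Settonotsimulate only stops simulation.
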(event `Set to simulate`
  (bind _returnvalue (`GameplayStatics.GetPlayerCharacter` 0))
  (bind _target_portal (`self.Target Portal`))
  (bind _target_portal_2 (`self.Target Portal`))
  (bind (_returnvalue_location _returnvalue_rotation) (`KismetMathLibrary.BreakTransform` (`self.GetTransform` _target_portal)))
  (bind (_returnvalue_location_2 _returnvalue_rotation_2) (`KismetMathLibrary.BreakTransform` (`self.GetTransform` _target_portal_2)))
  (`|ExecutionSequence` :!label _label
    (:`then_0`
      (bind _asfirst_person_character (cast `/Game/FirstPersonBP/Blueprints/FirstPersonCharacter` _returnvalue))
      (if (`self.Is exit Portal?`)
        (for _array_element (`self.Object Array`)
          (bind _astime_object (cast `/Game/Blueprints/Time_Objects/Time_Object` _array_element))
          (`PrimitiveComponent.SetSimulatePhysics` (`/Game/Blueprints/Time_Objects/Time_Object.StaticMesh` _astime_object) true)
          (`/Game/Blueprints/Time_Objects/Time_Object.Begin simulation` _astime_object))
        (else
          (`/Engine/EditorBlueprintResources/StandardMacros.IsValid` _target_portal
            (:`Is Valid`
              (`self.K2_SetActorLocationAndRotation` _asfirst_person_character _returnvalue_location _returnvalue_rotation false true)
              (bind _asfirst_person_character_2 (cast `/Game/FirstPersonBP/Blueprints/FirstPersonCharacter` (`GameplayStatics.GetPlayerCharacter` 0)))
              (set `/Game/FirstPersonBP/Blueprints/FirstPersonCharacter.Spawn Portal` (`self.Target Portal`) _asfirst_person_character_2)
              (for _array_element_2 (`self.Object Array`) :!label _label_2
                (bind _astime_object_2 (cast `/Game/Blueprints/Time_Objects/Time_Object` _array_element_2))
                (`PrimitiveComponent.SetSimulatePhysics` (`/Game/Blueprints/Time_Objects/Time_Object.StaticMesh` _astime_object_2) false)
                (`/Game/Blueprints/Time_Objects/Time_Object.End Simulation` _astime_object_2)))))))
    (:`then_1`
      (bind _asfirst_person_character_3 (cast `/Game/FirstPersonBP/Blueprints/FirstPersonCharacter` _returnvalue))
      (if (`self.Is exit Portal?`)
        (for _array_element_3 (`self.Hamsterball array`)
          (bind _ashamster_ball (cast `/Game/Blueprints/HamsterBall` _array_element_3))
          (`PrimitiveComponent.SetSimulatePhysics` (`/Game/Blueprints/HamsterBall.Sphere` _ashamster_ball) true)
          (`/Game/Blueprints/HamsterBall.Begin simulation` _ashamster_ball))
        (else
          (`/Engine/EditorBlueprintResources/StandardMacros.IsValid` _target_portal_2
            (:`Is Valid`
              (`self.K2_SetActorLocationAndRotation` _asfirst_person_character_3 _returnvalue_location_2 _returnvalue_rotation_2 false true)
              (bind _asfirst_person_character_4 (cast `/Game/FirstPersonBP/Blueprints/FirstPersonCharacter` (`GameplayStatics.GetPlayerCharacter` 0)))
              (set `/Game/FirstPersonBP/Blueprints/FirstPersonCharacter.Spawn Portal` (`self.Target Portal`) _asfirst_person_character_4)
              (for _array_element_4 (`self.Hamsterball array`) :!label _label_3
                (bind _ashamster_ball_2 (cast `/Game/Blueprints/HamsterBall` _array_element_4))
                (`PrimitiveComponent.SetSimulatePhysics` (`/Game/Blueprints/HamsterBall.Sphere` _ashamster_ball_2) false)
                (`/Game/Blueprints/HamsterBall.End Simulation` _ashamster_ball_2)))))))))

(event `self.Capsule.OnComponentBeginOverlap`
  (params (OverlappedComponent :type "PrimitiveComponent Object Reference") (OtherActor :type "Actor Object Reference") (OtherComp :type "PrimitiveComponent Object Reference") (OtherBodyIndex :type Integer) (bFromSweep :type Boolean) (SweepResult :type "HitResult Structure (by ref)"))
  (if (== OtherActor (`GameplayStatics.GetPlayerCharacter` 0))
    (goto _label)))

(event `Set to not simulate`
  (`|ExecutionSequence`
    (:`then_0`
      (goto _label_2))
    (:`then_1`
      (goto _label_3))))

(fn `UserConstructionScript`
  (bind _is_exit_portal_ (`self.Is exit Portal?`))
  (`ParticleSystemComponent.SetTemplate` (`self.ParticleSystem`) (select `bool` _is_exit_portal_ :`false` "/Game/Particles/Portal/Portal.Portal" :`true` "/Game/Particles/Portal/Portal_Exit.Portal_Exit" :!type "ParticleSystem Object Reference"))
  (`LightComponent.SetLightColor` (`self.PointLight`) (select `bool` _is_exit_portal_ :`false` (struct :`R` 0.796079 :`G` 0.423529 :`A` 1.0) :`true` (struct :`R` 1.0 :`G` 0.113725 :`B` 1.0 :`A` 1.0) :!type "LinearColor Structure") true))