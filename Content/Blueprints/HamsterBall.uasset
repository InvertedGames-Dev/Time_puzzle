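; Rideable hamster ball that the player enters or exits through Interact and that responds to time powers according to its ObjectType.
; Seat stays upright and carries the player; Door opens on approach.
; While simulation is enabled, rewindable types record rounded-deduplicated transforms and velocities (packed into transforms) for reverse playback, and stoppable types freeze physics.
; Materials reflect motion and time state, and falling too low resets the ball to its origin.
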(event `self.ReceiveTick`
  (params (DeltaSeconds :type "Float (single-precision)"))
  (bind _returnvalue (`GameplayStatics.GetPlayerCharacter` 0))
  (bind _seat (`self.Seat`))
  (`self.Tick 2`)
  (`self.Tick 3`)
  (`SceneComponent.K2_SetWorldRotation` :`self` _seat)
  (if (`self.Has Entered?`)
    (`SceneComponent.K2_SetWorldLocation` (`Actor.RootComponent` _returnvalue) (`SceneComponent.K2_GetComponentLocation` _seat) false true)
    (`PrimitiveComponent.SetCollisionEnabled` (`Character.CapsuleComponent` _returnvalue) "QueryOnly")))

(event `Tick 3`
  (bind _door (`self.Door`))
  (bind _asfirst_person_character (cast `/Game/FirstPersonBP/Blueprints/FirstPersonCharacter` (`GameplayStatics.GetPlayerCharacter` 0)))
  (if (`/Game/FirstPersonBP/Blueprints/FirstPersonCharacter.Is in ball?` _asfirst_person_character)
    (`SceneComponent.K2_SetRelativeLocationAndRotation` :`self` _door :`bSweep` true :!label _label)
    (elif (`self.Near Ball?`)
      (`SceneComponent.K2_SetRelativeLocationAndRotation` _door (43.0 0.0 0.0) (struct :`Pitch` 50.0) true false)
      (else
        (goto _label)))))

(event `Interact`
  (bind _returnvalue (`GameplayStatics.GetPlayerCharacter` 0))
  (if (`self.Has Entered?`)
    (set `self.Has Entered?` false)
    (`PrimitiveComponent.SetCollisionEnabled` (`Character.CapsuleComponent` _returnvalue) "QueryAndPhysics")
    (`SceneComponent.K2_SetWorldLocation` (`Actor.RootComponent` _returnvalue) (+ (`SceneComponent.K2_GetComponentLocation` (`self.Seat`)) (0.0 -200.0 0.0)) false true)
    (bind _asfirst_person_character (cast `/Game/FirstPersonBP/Blueprints/FirstPersonCharacter` (`GameplayStatics.GetPlayerCharacter` 0)))
    (set `/Game/FirstPersonBP/Blueprints/FirstPersonCharacter.Is in ball?` false _asfirst_person_character)
    (else
      (bind _output_get (set `self.Has Entered?` true))
      (bind _asfirst_person_character_2 (cast `/Game/FirstPersonBP/Blueprints/FirstPersonCharacter` (`GameplayStatics.GetPlayerCharacter` 0)))
      (set `/Game/FirstPersonBP/Blueprints/FirstPersonCharacter.Is in ball?` _output_get _asfirst_person_character_2)
      (`/Game/FirstPersonBP/Blueprints/FirstPersonCharacter.Drop Object` _asfirst_person_character_2))))

(event `self.ReceiveBeginPlay`
  (bind _asfirst_person_character (cast `/Game/FirstPersonBP/Blueprints/FirstPersonCharacter` (`GameplayStatics.GetPlayerCharacter` 0)))
  (set `self.Character Reference` _asfirst_person_character)
  (`PrimitiveComponent.SetSimulatePhysics` (`self.Sphere`) false))

(event `self.Interact Sphere.OnComponentBeginOverlap`
  (params (OverlappedComponent :type "PrimitiveComponent Object Reference") (OtherActor :type "Actor Object Reference") (OtherComp :type "PrimitiveComponent Object Reference") (OtherBodyIndex :type Integer) (bFromSweep :type Boolean) (SweepResult :type "HitResult Structure (by ref)"))
  (bind _asfirst_person_character (cast `/Game/FirstPersonBP/Blueprints/FirstPersonCharacter` OtherActor))
  (`/Game/UI/HUD.Event Show Use Text` (`/Game/FirstPersonBP/Blueprints/FirstPersonCharacter.Hud Reference` _asfirst_person_character))
  (set `/Game/FirstPersonBP/Blueprints/FirstPersonCharacter.Hamster Ball Reference` self _asfirst_person_character)
  (set `self.Near Ball?` true))

(event `self.Interact Sphere.OnComponentEndOverlap`
  (params (OverlappedComponent :type "PrimitiveComponent Object Reference") (OtherActor :type "Actor Object Reference") (OtherComp :type "PrimitiveComponent Object Reference") (OtherBodyIndex :type Integer))
  (bind _asfirst_person_character (cast `/Game/FirstPersonBP/Blueprints/FirstPersonCharacter` OtherActor))
  (`/Game/UI/HUD.Event Hide Use Text` (`/Game/FirstPersonBP/Blueprints/FirstPersonCharacter.Hud Reference` _asfirst_person_character))
  (set `/Game/FirstPersonBP/Blueprints/FirstPersonCharacter.Hamster Ball Reference` null _asfirst_person_character)
  (set `self.Near Ball?` false))

(event `Tick 2`
  (bind _character_reference (`self.Character Reference`))
  (bind _velocity_array (`self.Velocity Array`))
  (bind _transform_array (`self.Transform Array`))
  (bind _object_type (`self.Object type`))
  (bind _object_type_2 (`self.Object type`))
  (bind _sphere (`self.Sphere`))
  (bind _sphere_2 (`self.Sphere`))
  (bind _character_reference_2 (`self.Character Reference`))
  (bind _object_type_3 (`self.Object type`))
  (bind _object_type_4 (`self.Object type`))
  (bind _returnvalue (`KismetArrayLibrary.Array_LastIndex` _transform_array))
  (bind _returnvalue_2 (`KismetArrayLibrary.Array_LastIndex` _velocity_array))
  (bind _returnvalue_3 (`SceneComponent.K2_GetComponentToWorld` _sphere))
  (bind _stop_time (`/Game/FirstPersonBP/Blueprints/FirstPersonCharacter.Stop Time` _character_reference))
  (bind _reverse_time (`/Game/FirstPersonBP/Blueprints/FirstPersonCharacter.Reverse Time` _character_reference))
  (bind _output (`|GetArrayItem` _transform_array _returnvalue))
  (bind _returnvalue_4 (and _reverse_time (not _stop_time)))
  (`/Engine/EditorBlueprintResources/StandardMacros.Gate` true :!label _label_2
    (:`Exit`
      (set `self.Not moving` (and (`self.V not moving`) (`self.L not moving`)))
      (`|ExecutionSequence`
        (:`then_0`
          (if (or (`|EnumEquality` _object_type "NewEnumerator2") (`|EnumEquality` _object_type "NewEnumerator0"))
            (`|ExecutionSequence`
              (:`then_0`
                (if _returnvalue_4
                  (`SceneComponent.K2_SetWorldTransform` _sphere _output false false)
                  (if (> _returnvalue 0)
                    (`KismetArrayLibrary.Array_Remove` _transform_array _returnvalue))
                  (elif (and _stop_time (or (`|EnumEquality` _object_type_3 "NewEnumerator1") (`|EnumEquality` _object_type_3 "NewEnumerator0")))
                    _
                    (elif (`self.Compare rough transforms` _output _returnvalue_3)
                      (set `self.L not moving` true)
                      (else
                        (`KismetArrayLibrary.Array_Add` _transform_array _returnvalue_3)
                        (set `self.L not moving` false))))))
              (:`then_1`
                (if _returnvalue_4
                  (`PrimitiveComponent.SetPhysicsLinearVelocity` _sphere (.location (`|GetArrayItem` _velocity_array _returnvalue_2)) false "None")
                  (`PrimitiveComponent.SetPhysicsAngularVelocity` _sphere (.scale (`|GetArrayItem` _velocity_array _returnvalue_2)) false "None")
                  (if (> _returnvalue_2 0)
                    (`KismetArrayLibrary.Array_Remove` _velocity_array _returnvalue_2))
                  (elif (not _stop_time)
                    (bind _returnvalue_5 (`PrimitiveComponent.GetPhysicsLinearVelocity` _sphere "None"))
                    (bind _returnvalue_6 (`PrimitiveComponent.GetPhysicsAngularVelocity` _sphere "None"))
                    (bind _returnvalue_7 (`KismetMathLibrary.MakeTransform` _returnvalue_5 (struct) _returnvalue_6))
                    (if (`self.Compare rough transforms` (`|GetArrayItem` _velocity_array _returnvalue_2) _returnvalue_7)
                      (set `self.V not moving` true)
                      (else
                        (`KismetArrayLibrary.Array_Add` _velocity_array _returnvalue_7)
                        (set `self.V not moving` false)))))))))
        (:`then_1`
          (`PrimitiveComponent.SetMaterial` (`self.Main Ball`) 1 (select `bool` (or (`self.Not moving`) _reverse_time) :`false` (select `/Game/Blueprints/Time_Objects/Object_Type` _object_type_2 :`NewEnumerator0` "/Game/Blueprints/Time_Objects/Fragment_Active.Fragment_Active" :`NewEnumerator1` "/Game/Blueprints/Time_Objects/Freeze_Fragment_Dormant1.Freeze_Fragment_Dormant1" :`NewEnumerator2` "/Game/Blueprints/Time_Objects/Fragment_Active.Fragment_Active" :!type "Material Object Reference") :`true` (select `/Game/Blueprints/Time_Objects/Object_Type` _object_type_2 :`NewEnumerator0` "/Game/Blueprints/Time_Objects/U_Fragment_Dormant.U_Fragment_Dormant" :`NewEnumerator1` "/Game/Blueprints/Time_Objects/Freeze_Fragment_Dormant1.Freeze_Fragment_Dormant1" :`NewEnumerator2` "/Game/Blueprints/Time_Objects/Rewind_Fragment_Dormant.Rewind_Fragment_Dormant" :!type "Material Object Reference"))))
        (:`then_2`
          (bind _returnvalue_8 (`PrimitiveComponent.GetPhysicsLinearVelocity` (`self.Sphere`) "None"))
          (set `self.Velocity` _returnvalue_8)
          (if (or (`|EnumEquality` _object_type_4 "NewEnumerator1") (`|EnumEquality` _object_type_4 "NewEnumerator0"))
            (if (and (not (`/Game/FirstPersonBP/Blueprints/FirstPersonCharacter.Reverse Time` _character_reference_2)) (`/Game/FirstPersonBP/Blueprints/FirstPersonCharacter.Stop Time` _character_reference_2))
              (`PrimitiveComponent.SetSimulatePhysics` _sphere_2 false)
              (else
                (`PrimitiveComponent.SetSimulatePhysics` _sphere_2 true)))))
        (:`then_3`
          (`self.Reset if fallen off world`))))))

(event `Begin simulation`
  (goto _label_2 :!via `Open`))

(event `End Simulation`
  (goto _label_2 :!via `Close`))

(event `Reset`
  (bind _sphere (`self.Sphere`))
  (`PrimitiveComponent.SetSimulatePhysics` _sphere false)
  (`SceneComponent.K2_SetWorldTransform` (`self.Sphere`) (`self.Origin Transform`) false true)
  (`PrimitiveComponent.SetSimulatePhysics` _sphere true)
  (`KismetArrayLibrary.Array_Clear` (`self.Velocity Array`))
  (`KismetArrayLibrary.Array_Clear` (`self.Transform Array`)))

(fn `Compare Rough Transforms`
  (params (T1 :type "Transform Structure") (T2 :type "Transform Structure"))
  (returns (Equal :type Boolean))
  (return (and (and (== (`KismetMathLibrary.Round` (.x (.location T1))) (`KismetMathLibrary.Round` (.x (.location T2)))) (== (`KismetMathLibrary.Round` (.y (.location T1))) (`KismetMathLibrary.Round` (.y (.location T2)))) (== (`KismetMathLibrary.Round` (.z (.location T1))) (`KismetMathLibrary.Round` (.z (.location T2))))) (and (== (`KismetMathLibrary.Round` (.x (.scale T1))) (`KismetMathLibrary.Round` (.x (.scale T2)))) (== (`KismetMathLibrary.Round` (.y (.scale T1))) (`KismetMathLibrary.Round` (.y (.scale T2)))) (== (`KismetMathLibrary.Round` (.z (.scale T1))) (`KismetMathLibrary.Round` (.z (.scale T2))))))))

(fn `Reset if fallen off world`
  (bind _sphere (`self.Sphere`))
  (bind (_returnvalue_x _returnvalue_y _returnvalue_z) (`KismetMathLibrary.BreakVector` (`SceneComponent.K2_GetComponentLocation` (`self.Sphere`))))
  (if (<= _returnvalue_z 10.0)
    (`PrimitiveComponent.SetSimulatePhysics` _sphere false)
    (`SceneComponent.K2_SetWorldTransform` (`self.Sphere`) (`self.Origin Transform`) false true)
    (`PrimitiveComponent.SetSimulatePhysics` _sphere true)
    (`KismetArrayLibrary.Array_Clear` (`self.Velocity Array`))
    (`KismetArrayLibrary.Array_Clear` (`self.Transform Array`))))

(fn `UserConstructionScript`
  (bind _sphere (`self.Sphere`))
  (set `self.Origin Transform` (`SceneComponent.K2_GetComponentToWorld` _sphere))
  (`PrimitiveComponent.SetMaterial` _sphere 0 (select `/Game/Blueprints/Time_Objects/Object_Type` (`self.Object type`) :`NewEnumerator0` "/Game/Blueprints/Time_Objects/U_Fragment_Dormant.U_Fragment_Dormant" :`NewEnumerator1` "/Game/Blueprints/Time_Objects/Freeze_Fragment_Dormant1.Freeze_Fragment_Dormant1" :`NewEnumerator2` "/Game/Blueprints/Time_Objects/Rewind_Fragment_Dormant.Rewind_Fragment_Dormant" :!type "Material Object Reference"))
  (`SceneComponent.K2_SetRelativeLocationAndRotation` :`self` (`self.Door`) :`bSweep` true))