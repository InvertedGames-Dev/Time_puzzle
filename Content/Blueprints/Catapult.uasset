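; Catapult Blueprint that swings its arm up when triggered and lowers it back to rest when the trigger releases after firing finishes.
; The construction script sets the arm's resting pitch, and Fire and Reset each open a Gate.
; Tick feeds both Gates to step CatapultArm's pitch a fixed amount per frame, without delta-time scaling.
; Truncated angle checks trigger DoOnce nodes that close each Gate at its end position.
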(event `Fire`
  (`|ExecutionSequence`
    (:`then_0`
      (goto _label_4 :!via `Reset`))
    (:`then_1`
      (goto _label_5 :!via `Open`))))

(event `Set up`)

(event `self.ReceiveTick`
  (params (DeltaSeconds :type "Float (single-precision)"))
  (if (`self.Reset?`)
    (`self.Reset`)
    (if (== (`KismetMathLibrary.FTrunc` (`self.Current Rotation`)) -70) :!label _label
      (`/Engine/EditorBlueprintResources/StandardMacros.DoOnce` false :!label _label_2
        (:`Completed`
          (set `self.Reset?` false)
          (goto _label_3 :!via `Close`)))
      (else
        (`/Engine/EditorBlueprintResources/StandardMacros.Gate` true :!label _label_3
          (:`Exit`
            (bind _output_get (set `self.Current Rotation` (+ (`self.Current Rotation`) -2.0)))
            (`SceneComponent.K2_SetRelativeRotation` (`self.CatapultArm`) (`KismetMathLibrary.MakeRotator` 0.0 _output_get) false false)))))
    (else
      (`|ExecutionSequence`
        (:`then_0`
          (if (== (`KismetMathLibrary.FTrunc` (`self.Current Rotation`)) -24)
            (`/Engine/EditorBlueprintResources/StandardMacros.DoOnce` false :!label _label_4
              (:`Completed`
                (set `self.Done firing` true)
                (goto _label_5 :!via `Close`)))
            (else
              (set `self.Done firing` false)
              (`/Engine/EditorBlueprintResources/StandardMacros.Gate` true :!label _label_5
                (:`Exit`
                  (bind _output_get_2 (set `self.Current Rotation` (+ (`self.Current Rotation`) 2.0)))
                  (`SceneComponent.K2_SetRelativeRotation` (`self.CatapultArm`) (`KismetMathLibrary.MakeRotator` 0.0 _output_get_2) false false))))))
        (:`then_1`
          (goto _label))))))

(event `Reset`
  (`|ExecutionSequence`
    (:`then_0`
      (goto _label_2 :!via `Reset`))
    (:`then_1`
      (goto _label_3 :!via `Open`))))

(event `/Game/Blueprints/Triggers/BPI_Trigger.Trigger On`
  (`self.Fire`))

(event `/Game/Blueprints/Triggers/BPI_Trigger.Trigger Off`
  (if (`self.Done firing`)
    (`self.Reset`)))

(fn `UserConstructionScript`
  (`SceneComponent.K2_SetRelativeRotation` (`self.CatapultArm`) (struct :`Pitch` -70.0) false false))