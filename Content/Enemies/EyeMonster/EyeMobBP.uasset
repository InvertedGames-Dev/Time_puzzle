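; Eye monster enemy that turns to face the player and fires laser beams.
; Tick drives a gated yaw-tracking step, and pawn sensing drives a gated Attack that briefly raises IsShooting while the player lives.
; A separate Shoot event spawns LaserBeamBP at the arrow, then again after a delay unless the player is dead.
; StopForAMoment shuts both gates for two seconds, and tracking calls it when the player is dead.
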(event `Stop for a moment`
  (bind _returnvalue (`self.K2_GetActorLocation`))
  (`|ExecutionSequence`
    (:`then_0`
      (goto _label :!via `Close`))
    (:`then_1`
      (goto _label_2 :!via `Close`))
    (:`then_2`
      (`KismetSystemLibrary.Delay` 2.0)
      (`|ExecutionSequence`
        (:`then_0`
          (goto _label_2 :!via `Open`))
        (:`then_1`
          (goto _label :!via `Open`))))))

(event `self.ReceiveTick`
  (params (DeltaSeconds :type "Float (single-precision)"))
  (bind _returnvalue (`self.K2_GetActorLocation`))
  (`/Engine/EditorBlueprintResources/StandardMacros.Gate` false :!label _label
    (:`Exit`
      (bind _asfirst_person_character (cast `/Game/FirstPersonBP/Blueprints/FirstPersonCharacter` (`GameplayStatics.GetPlayerCharacter` 0)))
      (if (`/Game/FirstPersonBP/Blueprints/FirstPersonCharacter.Is dead?` _asfirst_person_character)
        (`self.Stop for a moment`)
        (else
          (bind (_returnvalue_roll _returnvalue_pitch) (`KismetMathLibrary.BreakRotator` (`self.K2_GetActorRotation` (stale `self.PawnSensing.OnSeePawn` _asfirst_person_character))))
          (bind (_returnvalue_roll_2 _returnvalue_pitch_2 _returnvalue_yaw) (`KismetMathLibrary.BreakRotator` (`KismetMathLibrary.FindLookAtRotation` _returnvalue (`self.K2_GetActorLocation` (stale `self.PawnSensing.OnSeePawn` _asfirst_person_character)))))
          (`self.K2_SetActorTransform` (`KismetMathLibrary.MakeTransform` _returnvalue (`KismetMathLibrary.MakeRotator` _returnvalue_roll _returnvalue_pitch _returnvalue_yaw)) true))))))

(event `self.PawnSensing.OnSeePawn`
  (params (Pawn :type "Pawn Object Reference"))
  (`/Engine/EditorBlueprintResources/StandardMacros.Gate` false :!label _label_2
    (:`Exit`
      (bind _asfirst_person_character (cast `/Game/FirstPersonBP/Blueprints/FirstPersonCharacter` Pawn))
      (if (not (`/Game/FirstPersonBP/Blueprints/FirstPersonCharacter.Is dead?` _asfirst_person_character))
        (`self.Attack`)))))

(event `Attack`
  (set `self.IsShooting` true)
  (`KismetSystemLibrary.Delay` 1.3)
  (set `self.IsShooting` false))

(event `Shoot`
  (bind _returnvalue (`SceneComponent.K2_GetComponentToWorld` (`self.Arrow1`)))
  (`|SpawnActorFromClass` "/Game/Enemies/EyeMonster/LaserBeamBP.LaserBeamBP_C" _returnvalue "Undefined" "OverrideRootScale" null null)
  (`KismetSystemLibrary.Delay` (`self.Delay Between Shots`))
  (if (not (`/Game/FirstPersonBP/Blueprints/FirstPersonCharacter.Is dead?` (stale `self.ReceiveTick` _asfirst_person_character)))
    (`|SpawnActorFromClass` "/Game/Enemies/EyeMonster/LaserBeamBP.LaserBeamBP_C" _returnvalue "Undefined" "OverrideRootScale" null null)))

(fn `UserConstructionScript`)